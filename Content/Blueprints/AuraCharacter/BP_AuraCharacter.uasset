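; Player character Blueprint for Aura, handling attack facing, camera-obstruction fading and ability voice lines.
; Facing target updates feed a Motion Warping warp target named FacingTarget.
; CollBox overlaps send fade out and fade in messages to actors implementing BI_FadeInterface.
; Triggered ability tags for the fire and lightning spells are matched exactly to play Aura's 2D voice sounds.
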(event `SetFacingTarget`
  (params (FacingTarget :type "Vector Structure"))
  (`MotionWarpingComponent.AddOrUpdateWarpTargetFromLocation` (`self.MotionWarping`) "FacingTarget" FacingTarget))

(event `CombatInterface.UpdateFacingTarget`
  (params (Target :type "Vector Structure (by ref)"))
  (`self.SetFacingTarget` Target))

(event `self.CollBox.OnComponentBeginOverlap`
  (params (OverlappedComponent :type "PrimitiveComponent Object Reference") (OtherActor :type "Actor Object Reference") (OtherComp :type "PrimitiveComponent Object Reference") (OtherBodyIndex :type Integer) (bFromSweep :type Boolean) (SweepResult :type "HitResult Structure (by ref)"))
  (if (`KismetSystemLibrary.DoesImplementInterface` OtherActor "/Game/Blueprints/Actors/FadeActor/BI_FadeInterface.BI_FadeInterface_C")
    (message `/Game/Blueprints/Actors/FadeActor/BI_FadeInterface.Fade Out` OtherActor)))

(event `self.CollBox.OnComponentEndOverlap`
  (params (OverlappedComponent :type "PrimitiveComponent Object Reference") (OtherActor :type "Actor Object Reference") (OtherComp :type "PrimitiveComponent Object Reference") (OtherBodyIndex :type Integer))
  (if (`KismetSystemLibrary.DoesImplementInterface` OtherActor "/Game/Blueprints/Actors/FadeActor/BI_FadeInterface.BI_FadeInterface_C")
    (message `/Game/Blueprints/Actors/FadeActor/BI_FadeInterface.Fade In` OtherActor)))

(event `self.OnAbilityVoiceTriggered`
  (params (AbilityTag :type "GameplayTag Structure"))
  (if (`BlueprintGameplayTagLibrary.MatchesTag` AbilityTag (struct :`TagName` "Abilities.Fire.FireBolt") true)
    (`GameplayStatics.PlaySound2D` "/Game/Assets/Sounds/Aura/sfx_Firebolt_Aura.sfx_Firebolt_Aura" 1.0 1.0 0.0 null null)
    (elif (`BlueprintGameplayTagLibrary.MatchesTag` AbilityTag (struct :`TagName` "Abilities.Fire.FireNado") true)
      (`GameplayStatics.PlaySound2D` "/Game/Assets/Sounds/Aura/sfx_FireNado_Aura.sfx_FireNado_Aura" 1.0 1.0 0.0 null null)
      (elif (`BlueprintGameplayTagLibrary.MatchesTag` AbilityTag (struct :`TagName` "Abilities.Lightning.Electrocute") true)
        (`GameplayStatics.PlaySound2D` "/Game/Assets/Sounds/Aura/sfx_Shock_Aura.sfx_Shock_Aura" 1.0 1.0 0.0 null null)
        (elif (`BlueprintGameplayTagLibrary.MatchesTag` AbilityTag (struct :`TagName` "Abilities.Fire.DelayedBlast") true)
          (`GameplayStatics.PlaySound2D` "/Game/Assets/Sounds/Aura/sfx_DelayBlast_Aura.sfx_DelayBlast_Aura" 1.0 1.0 0.0 null null))))))

(fn `UserConstructionScript`)