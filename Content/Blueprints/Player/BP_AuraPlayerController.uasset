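; BP_AuraPlayerController is a player controller that handles the in-game settings menu and the exit to the load menu level.
; The IA_Esc input toggles WBP_SettingMenu, creating it and pausing the game, or calling CloseSetttingMenu to remove it, clear the reference and unpause.
; QuitToLoadScreen unpauses and opens the LoadMenu level by object reference.
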(event `EnhancedInput|/Game/Blueprints/Input/InputActions/IA_Esc`
  (params (ActionValue :type Boolean) (ElapsedSeconds :type "Float (double-precision)") (TriggeredSeconds :type "Float (double-precision)") (InputAction :type "InputAction Object Reference" :default "/Game/Blueprints/Input/InputActions/IA_Esc.IA_Esc"))
  (:`Started`
    (`/Engine/EditorBlueprintResources/StandardMacros.IsValid` (`self.SettingMenu`)
      (:`Is Valid`
        (`self.CloseSetttingMenu`))
      (:`Is Not Valid`
        (bind _returnvalue (`|CreateWidget` "/Game/Blueprints/UI/SettingsMenu/WBP_SettingMenu.WBP_SettingMenu_C" self))
        (bind _output_get (set `self.SettingMenu` _returnvalue))
        (`UserWidget.AddToViewport` _output_get 0)
        (`GameplayStatics.SetGamePaused` true)))))

(fn `CloseSetttingMenu`
  (`Widget.RemoveFromParent` (`self.SettingMenu`))
  (set `self.SettingMenu` null)
  (`GameplayStatics.SetGamePaused` false))

(fn `QuitToLoadScreen`
  (`GameplayStatics.SetGamePaused` false)
  (`GameplayStatics.OpenLevelBySoftObjectPtr` "/Game/Maps/LoadMenu.LoadMenu"))

(fn `UserConstructionScript`)