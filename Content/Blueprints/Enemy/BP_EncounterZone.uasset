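; Encounter zone actor that keeps its assigned enemies dormant until the Aura player character enters its box.
; On BeginPlay it stops the brain component logic on each enemy's BP_AuraAIController.
; The first box overlap by a BP_AuraCharacter passes a DoOnce and restarts that logic for every valid enemy in the Enemies array, with no deactivation afterward.
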(event `self.ReceiveBeginPlay`
  (for _array_element (`self.Enemies`)
    (`/Engine/EditorBlueprintResources/StandardMacros.IsValid` _array_element
      (:`Is Valid`
        (bind _asbp_aura_aicontroller (cast `/Game/Blueprints/AI/AIController/BP_AuraAIController` (`Pawn.GetController` _array_element)))
        (bind _braincomponent (`AIController.BrainComponent` _asbp_aura_aicontroller))
        (`/Engine/EditorBlueprintResources/StandardMacros.IsValid` _braincomponent
          (:`Is Valid`
            (`BrainComponent.StopLogic` _braincomponent "Encounter Inactive")))))))

(event `self.Box.OnComponentBeginOverlap`
  (params (OverlappedComponent :type "PrimitiveComponent Object Reference") (OtherActor :type "Actor Object Reference") (OtherComp :type "PrimitiveComponent Object Reference") (OtherBodyIndex :type Integer) (bFromSweep :type Boolean) (SweepResult :type "HitResult Structure (by ref)"))
  (cast `/Game/Blueprints/AuraCharacter/BP_AuraCharacter` OtherActor)
  (`/Engine/EditorBlueprintResources/StandardMacros.DoOnce` false
    (:`Completed`
      (for _array_element (`self.Enemies`)
        (`/Engine/EditorBlueprintResources/StandardMacros.IsValid` _array_element
          (:`Is Valid`
            (bind _returnvalue (`Pawn.GetController` _array_element))
            (`/Engine/EditorBlueprintResources/StandardMacros.IsValid` _returnvalue
              (:`Is Valid`
                (bind _asbp_aura_aicontroller (cast `/Game/Blueprints/AI/AIController/BP_AuraAIController` _returnvalue))
                (bind _braincomponent (`AIController.BrainComponent` _asbp_aura_aicontroller))
                (`/Engine/EditorBlueprintResources/StandardMacros.IsValid` _braincomponent
                  (:`Is Valid`
                    (`BrainComponent.RestartLogic` _braincomponent)))))))))))

(fn `UserConstructionScript`)