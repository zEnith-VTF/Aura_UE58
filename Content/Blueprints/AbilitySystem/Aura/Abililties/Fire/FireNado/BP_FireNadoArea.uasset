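; BP_FireNadoArea is the area actor for the Fire Nado ability, keeping its VFX sized to the area's configured radius.
; On OnAreaConfigured, it caches the AreaVFX component's original relative scale the first time only.
; It then scales that cached value uniformly by Radius over BaseVisualRadius, so repeated configuration does not compound the scale.
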(event `self.OnAreaConfigured`
  (params (Radius :type "Float (single-precision)"))
  (bind _areavfx (`self.AreaVFX`))
  (bind _returnvalue (`KismetMathLibrary.SafeDivide` Radius (`self.BaseVisualRadius`)))
  (`|ExecutionSequence`
    (:`then_0`
      (`/Engine/EditorBlueprintResources/StandardMacros.DoOnce` false
        (:`Completed`
          (set `self.CachedBaseVisualScale` (`SceneComponent.RelativeScale3D` _areavfx)))))
    (:`then_1`
      (`SceneComponent.SetRelativeScale3D` _areavfx (* (`self.CachedBaseVisualScale`) (`KismetMathLibrary.MakeVector` _returnvalue _returnvalue _returnvalue))))))

(fn `UserConstructionScript`)