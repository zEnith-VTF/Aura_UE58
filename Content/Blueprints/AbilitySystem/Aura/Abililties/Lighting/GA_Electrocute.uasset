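; Channeled chain-lightning gameplay ability that electrocutes the target under the mouse and additional targets while input is held.
; On activation it gathers targets, starts a looping shock sound and spawns beams from the weapon tip to the hit point, branching to the others.
; Looping timers reposition the beams and apply authority-only damage ticks.
; Input release or primary target death ends it, while secondary deaths call for removing that target's beam.
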(event `self.K2_ActivateAbility`
  (bind _mousehitactor (`self.MouseHitActor`))
  (bind _ownercharacter (`self.OwnerCharacter`))
  (`self.K2_CommitAbility`)
  (bind _returnvalue (`GameplayStatics.SpawnSound2D` "/Game/Assets/Sounds/Abilities/Shock/sfx_ShockLoop.sfx_ShockLoop" 1.0 1.0 0.0 null))
  (set `self.ChainLightningAudioComponent` _returnvalue)
  (bind (_asynctaskproxy _data) (`TargetDataUnderMouse.CreateTargetDataUnderMouse` false)
    (:`ValidData`
      (`self.StoreMouseDataInfo` (`AbilitySystemBlueprintLibrary.GetHitResultFromTargetData` _data))
      (`self.StoreOwnerVariables`)
      (`self.TraceFirstTarget` (`self.MouseHitLocation`))
      (bind _outadditionaltargets (`self.StoreAdditionalTargets`))
      (set `self.AdditionalTargets` _outadditionaltargets)
      (`self.SpawnBeams`)
      (bind _returnvalue_2 (`KismetSystemLibrary.K2_SetTimer` self "DamageTick" (`self.DamageTickInterval`) true))
      (`|ExecutionSequence`
        (:`then_0`
          (`/Engine/EditorBlueprintResources/StandardMacros.IsValid` _mousehitactor
            (:`Is Valid`
              (`/Engine/EditorBlueprintResources/StandardMacros.IsValid` _ownercharacter
                (:`Is Valid`
                  (bind _returnvalue_3 (message `CombatInterface.GetWeapon` _ownercharacter))
                  (`/Engine/EditorBlueprintResources/StandardMacros.IsValid` _returnvalue_3
                    (:`Is Valid`
                      (if (`KismetSystemLibrary.DoesImplementInterface` _mousehitactor "/Script/Aura.CombatInterface")
                        (bind _returnvalue_4 (message `CombatInterface.IsDead` _mousehitactor))
                        (if (not _returnvalue_4)
                          (if (`KismetSystemLibrary.K2_IsTimerActiveHandle` _returnvalue_2) :!label _label
                            (`self.ReportSuccessfulCastForVoice`)))
                        (else
                          (goto _label))))))))))
        (:`then_1`
          (`KismetSystemLibrary.K2_SetTimer` self "UpdateBeams" 0.02 true)
          (`AbilityTask_WaitInputRelease.WaitInputRelease` true
            (:`OnRelease`
              (`self.EndElectrocute`))))))))

(event `self.PrimaryTargetDied`
  (params (DeadActor :type "Actor Object Reference"))
  (`self.EndElectrocute`))

(event `self.AdditionalTargetDied`
  (params (DeadActor :type "Actor Object Reference"))
  (`self.RemoveBeamForTarget` DeadActor))

(event `self.K2_OnEndAbility`
  (params (bWasCancelled :type Boolean))
  (`/Engine/EditorBlueprintResources/StandardMacros.IsValid` (`self.ChainLightningAudioComponent`)
    (:`Is Valid`
      (`AudioComponent.Stop` (`self.ChainLightningAudioComponent`)))
    (:`Is Not Valid`
      _))
  (set `self.ChainLightningAudioComponent` null))

(fn `DamageTick`
  (bind _mousehitactor (`self.MouseHitActor`))
  (`self.K2_HasAuthority`
    (:`True`
      (for _array_element (`self.AdditionalTargets`)
        (`self.CauseDamage` _array_element))
      (`/Engine/EditorBlueprintResources/StandardMacros.IsValid` _mousehitactor
        (:`Is Valid`
          (`self.CauseDamage` _mousehitactor))))))

(fn `DestroyBeams`
  (bind _primarybeamcomponent (`self.PrimaryBeamComponent`))
  (for _array_element (`self.AdditionalBeamComponents`)
    (`ActorComponent.K2_DestroyComponent` _array_element))
  (`/Engine/EditorBlueprintResources/StandardMacros.IsValid` _primarybeamcomponent
    (:`Is Valid`
      (`ActorComponent.K2_DestroyComponent` _primarybeamcomponent))))

(fn `EndElectrocute`
  (`KismetSystemLibrary.K2_ClearTimer` self "DamageTick")
  (`KismetSystemLibrary.K2_ClearTimer` self "UpdateBeams")
  (`self.DestroyBeams`)
  (`self.K2_EndAbility`))

(fn `RemoveBeamForTarget`
  (params (DeadActor :type "Actor Object Reference"))
  (bind _returnvalue (`KismetArrayLibrary.Array_Find` (`self.AdditionalTargets`) DeadActor))
  (bind _output (`|GetArrayItem` (`self.AdditionalBeamComponents`) _returnvalue))
  (if (>= _returnvalue 0)
    (`KismetArrayLibrary.Array_Remove` (`self.AdditionalTargets`) _returnvalue)
    (`KismetArrayLibrary.Array_Remove` (`self.AdditionalBeamComponents`) _returnvalue)
    (`/Engine/EditorBlueprintResources/StandardMacros.IsValid` _output
      (:`Is Valid`
        (`ActorComponent.K2_DestroyComponent` _output)))))

(fn `SpawnBeams`
  (bind _returnvalue (message `CombatInterface.GetWeapon` (`self.OwnerCharacter`)))
  (`/Engine/EditorBlueprintResources/StandardMacros.IsValid` _returnvalue
    (:`Is Valid`
      (bind _returnvalue_2 (`NiagaraFunctionLibrary.SpawnSystemAtLocation` (`self.BeamSystem`) (`SceneComponent.GetSocketLocation` _returnvalue "TipSocket") (struct) (1.0 1.0 1.0) false))
      (set `self.PrimaryBeamComponent` _returnvalue_2)
      (for _ (`self.AdditionalTargets`)
        (bind _returnvalue_3 (`NiagaraFunctionLibrary.SpawnSystemAtLocation` (`self.BeamSystem`) (`Actor.K2_GetActorLocation` (`self.MouseHitActor`)) (struct) (1.0 1.0 1.0) false))
        (`KismetArrayLibrary.Array_AddUnique` (`self.AdditionalBeamComponents`) _returnvalue_3))
      (`self.UpdateBeams`))))

(fn `UpdateBeams`
  (bind _mousehitlocation (`self.MouseHitLocation`))
  (bind _primarybeamcomponent (`self.PrimaryBeamComponent`))
  (bind _returnvalue (message `CombatInterface.GetWeapon` (`self.OwnerCharacter`)))
  (`/Engine/EditorBlueprintResources/StandardMacros.IsValid` _returnvalue
    (:`Is Valid`
      (for _index (range (+ (- (`KismetArrayLibrary.Array_Length` (`self.AdditionalTargets`)) 1) 1))
        (bind _output (`|GetArrayItem` (`self.AdditionalBeamComponents`) _index))
        (`SceneComponent.K2_SetWorldLocation` _output _mousehitlocation false false)
        (bind _returnvalue_2 (`Actor.K2_GetActorLocation` (`|GetArrayItem` (`self.AdditionalTargets`) _index)))
        (`SceneComponent.K2_SetWorldRotation` _output (`KismetMathLibrary.FindLookAtRotation` _mousehitlocation _returnvalue_2) false false)
        (`NiagaraComponent.SetVariablePosition` _output "User.Beam Start" _returnvalue_2)
        (`NiagaraComponent.SetVariablePosition` _output "User.Beam End" _mousehitlocation))
      (`/Engine/EditorBlueprintResources/StandardMacros.IsValid` _primarybeamcomponent
        (:`Is Valid`
          (bind _returnvalue_3 (`SceneComponent.GetSocketLocation` _returnvalue "TipSocket"))
          (`SceneComponent.K2_SetWorldLocation` _primarybeamcomponent _returnvalue_3 false false)
          (`SceneComponent.K2_SetWorldRotation` _primarybeamcomponent (`KismetMathLibrary.FindLookAtRotation` _returnvalue_3 _mousehitlocation) false false)
          (`NiagaraComponent.SetVariablePosition` _primarybeamcomponent "User.Beam Start" _mousehitlocation)
          (`NiagaraComponent.SetVariablePosition` _primarybeamcomponent "User.Beam End" _returnvalue_3))))))