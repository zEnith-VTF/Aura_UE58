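; Shaman enemy summon ability that spawns random minion classes at shuffled spawn locations marked with ground-summon Niagara effects.
; While the summon montage plays, a delayed loop spawns minions one by one on the authority, facing away from the caster.
; Each minion must register with the AuraEnemy caster before getting a controller.
; Death, failure or montage interruption cancels; the ability ends once montage and batch both finish.
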(event `self.K2_ActivateAbility`
  (bind _returnvalue (`self.GetAvatarActorFromActorInfo`))
  (bind _returnvalue_2 (+ (`|GetArrayItem` (`self.Spawn Location`) (`self.SpawnLocationIndex`)) (0.0 0.0 70.0)))
  (bind _returnvalue_3 (`self.GetSpawnLocations`))
  (bind _output_get (set `self.Spawn Location` _returnvalue_3))
  (`KismetArrayLibrary.Array_Shuffle` _output_get)
  (for _array_element _output_get
    (`NiagaraFunctionLibrary.SpawnSystemAtLocation` "/Game/Assets/Effects/Combat/NS_GroundSummon.NS_GroundSummon" _array_element))
  (`AbilityTask_PlayMontageAndWait.CreatePlayMontageAndWaitProxy` "None" "/Game/Assets/Enemies/Shaman/Animations/AM_Shaman_Summon.AM_Shaman_Summon"
    (:`then`
      (`AbilityTask_WaitDelay.WaitDelay` 0.4
        (:`OnFinish`
          (if (< (`self.SpawnLocationIndex`) (`KismetArrayLibrary.Array_Length` (`self.Spawn Location`))) :!label _label
            (`/Engine/EditorBlueprintResources/StandardMacros.IsValid` _returnvalue
              (:`Is Valid`
                (bind _returnvalue_4 (message `CombatInterface.IsDead` _returnvalue))
                (if (not _returnvalue_4)
                  (`self.K2_HasAuthority`
                    (:`True`
                      (bind _returnvalue_5 (`|SpawnActorFromClass` (`self.GetRandomMinionClass`) (`KismetMathLibrary.MakeTransform` _returnvalue_2 (`KismetMathLibrary.FindLookAtRotation` (`Actor.K2_GetActorLocation` (`self.GetAvatarActorFromActorInfo`)) _returnvalue_2)) "AlwaysSpawn" "MultiplyWithRoot" null null))
                      (`/Engine/EditorBlueprintResources/StandardMacros.IsValid` _returnvalue_5
                        (:`Is Valid`
                          (bind _asaura_enemy (cast `AuraEnemy` _returnvalue)
                            (:`then`
                              (bind _returnvalue_6 (`AuraEnemy.RegisterSummonedMinion` _asaura_enemy _returnvalue_5))
                              (if _returnvalue_6
                                (`Pawn.SpawnDefaultController` _returnvalue_5)
                                (`/Engine/EditorBlueprintResources/StandardMacros.IncrementInt` (`self.SpawnLocationIndex`)
                                  (:`  `
                                    (`AbilityTask_WaitDelay.WaitDelay` 0.5
                                      (:`OnFinish`
                                        (goto _label)))))
                                (else
                                  _)))
                            (:`CastFailed`
                              _))
                          (`Actor.K2_DestroyActor` _returnvalue_5))
                        (:`Is Not Valid`
                          _)))
                    (:`False`
                      _))))
              (:`Is Not Valid`
                _))
            (`self.K2_CancelAbility` :!label _label_2)
            (else
              (set `self.bSummonBatchCompleted` true)
              (if (`self.bSummonMontageCompleted`) :!label _label_3
                (if (`self.bSummonBatchCompleted`)
                  (`self.K2_EndAbility`))))))))
    (:`OnCompleted`
      (set `self.bSummonMontageCompleted` true)
      (goto _label_3))
    (:`OnInterrupted`
      (goto _label_2))
    (:`OnCancelled`
      (goto _label_2))))

(event `OnDestroyed_事件`
  (params (DestroyedActor :type "Actor Object Reference")))