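; Enemy ranged attack ability that fires a projectile at the avatar's combat target.
; On activation it turns the avatar toward the target and plays a random tagged attack montage at increased rate.
; The montage's gameplay event tag times the shot, re-fetching the target and spawning the projectile from the montage's tagged socket.
; The ability ends when the montage completes or a target check fails; other montage outcomes are not wired.
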(event `self.K2_ActivateAbility`
  (bind _returnvalue (`self.GetAvatarActorFromActorInfo`))
  (bind _returnvalue_2 (message `EnemyInterface.GetCombatTarget` _returnvalue))
  (`/Engine/EditorBlueprintResources/StandardMacros.IsValid` _returnvalue_2
    (:`Is Valid`
      (message `CombatInterface.UpdateFacingTarget` _returnvalue (`Actor.K2_GetActorLocation` _returnvalue_2))
      (bind _returnvalue_3 (message `CombatInterface.GetAttackMontages` _returnvalue))
      (bind _output_get (set `self.Tagged Montage` (`self.GetRandomTaggedMontageFromArray` _returnvalue_3)))
      (bind (_montage _montagetag _sockettag) (break `TaggedMontage` _output_get))
      (`AbilityTask_PlayMontageAndWait.CreatePlayMontageAndWaitProxy` "None" _montage 2.0 "None" false
        (:`then`
          (`AbilityTask_WaitGameplayEvent.WaitGameplayEvent` _montagetag null true
            (:`EventReceived`
              (message `CombatInterface.GetCombatSocketLocation` (`self.GetAvatarActorFromActorInfo`) _sockettag)
              (bind _returnvalue_4 (message `EnemyInterface.GetCombatTarget` (`self.GetAvatarActorFromActorInfo`)))
              (`/Engine/EditorBlueprintResources/StandardMacros.IsValid` _returnvalue_4
                (:`Is Valid`
                  (`self.SpawnProjectile` (`Actor.K2_GetActorLocation` _returnvalue_4) _sockettag))
                (:`Is Not Valid`
                  (`self.K2_EndAbility`))))))
        (:`OnCompleted`
          (`self.K2_EndAbility`))))
    (:`Is Not Valid`
      (`self.K2_EndAbility`))))