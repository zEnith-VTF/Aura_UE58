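; Enemy melee attack Gameplay Ability that cancels if the avatar is invalid or dead and ends if it has no combat target.
; It turns the avatar toward the target and plays a random tagged attack montage.
; The montage's event tag triggers a sphere check at its combat socket, damaging non-friendly live players and firing a tagged MeleeImpact gameplay cue.
; The ability ends when the montage completes, is interrupted or is cancelled.
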(event `self.K2_ActivateAbility`
  (bind _returnvalue (`self.GetAvatarActorFromActorInfo`))
  (bind _returnvalue_2 (`self.GetAvatarActorFromActorInfo`))
  (`/Engine/EditorBlueprintResources/StandardMacros.IsValid` _returnvalue
    (:`Is Valid`
      (bind _returnvalue_3 (message `CombatInterface.IsDead` _returnvalue))
      (if _returnvalue_3
        (`self.K2_CancelAbility` :!label _label)
        (else
          (bind _returnvalue_4 (message `EnemyInterface.GetCombatTarget` _returnvalue))
          (`/Engine/EditorBlueprintResources/StandardMacros.IsValid` _returnvalue_4
            (:`Is Valid`
              (bind _ascombat_interface (cast `CombatInterface` _returnvalue))
              (`CombatInterface.UpdateFacingTarget` _ascombat_interface (`Actor.K2_GetActorLocation` _returnvalue_4))
              (bind _returnvalue_5 (message `CombatInterface.GetAttackMontages` (`self.GetAvatarActorFromActorInfo`)))
              (bind _output_get (set `self.TaggedMontaged` (`self.GetRandomTaggedMontageFromArray` _returnvalue_5)))
              (bind (_montage _montagetag _sockettag) (break `TaggedMontage` _output_get))
              (`AbilityTask_PlayMontageAndWait.CreatePlayMontageAndWaitProxy` "None" _montage
                (:`then`
                  (`AbilityTask_WaitGameplayEvent.WaitGameplayEvent` _montagetag null true
                    (:`EventReceived`
                      (`/Engine/EditorBlueprintResources/StandardMacros.IsValid` _returnvalue_2
                        (:`Is Valid`
                          (bind _returnvalue_6 (message `CombatInterface.IsDead` _returnvalue_2))
                          (if _returnvalue_6
                            (`self.K2_CancelAbility` :!label _label_2)
                            (else
                              (bind _returnvalue_7 (message `CombatInterface.GetCombatSocketLocation` _returnvalue_2 _sockettag))
                              (bind _outoverlappingactors (`AuraAbilitySystemLibrary.GetLivePlayersWithinRadius` _returnvalue_2 (`|MakeArray` _returnvalue_2) 100.0 _returnvalue_7))
                              (for _array_element _outoverlappingactors
                                (`/Engine/EditorBlueprintResources/StandardMacros.IsValid` _array_element
                                  (:`Is Valid`
                                    (if (not (`AuraAbilitySystemLibrary.AreActorsFriends` (`self.GetAvatarActorFromActorInfo`) _array_element))
                                      (`self.CauseDamage` _array_element)
                                      (`self.K2_ExecuteGameplayCueWithParams` (struct :`TagName` "GameplayCue.MeleeImpact") (`AbilitySystemBlueprintLibrary.MakeGameplayCueParameters` 0.0 0.0 (struct) (struct) (struct) (`BlueprintGameplayTagLibrary.MakeGameplayTagContainerFromTag` (`.MontageTag` (break `TaggedMontage` (`self.TaggedMontaged`)))) (struct) (`Actor.K2_GetActorLocation` _array_element) (0.0 0.0 0.0) null (`self.GetAvatarActorFromActorInfo`) _array_element)))))))))
                        (:`Is Not Valid`
                          (goto _label_2))))))
                (:`OnCompleted`
                  (`self.K2_EndAbility` :!label _label_3))
                (:`OnInterrupted`
                  (goto _label_3))
                (:`OnCancelled`
                  (goto _label_3))))
            (:`Is Not Valid`
              (`self.K2_EndAbility`))))))
    (:`Is Not Valid`
      (goto _label))))