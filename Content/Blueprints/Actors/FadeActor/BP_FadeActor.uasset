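; BP_FadeActor is a static mesh actor that fades through a material parameter via FadeOut and Fadein events.
; Its construction script caches the original materials and creates dynamic instances from a list of fade materials.
; FadeOut applies those instances by slot and plays a timeline driving their "Fade" scalar; Fadein reverses it.
; When the timeline finishes at 1 or above, the original materials are restored.
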(event `/Game/Blueprints/Actors/FadeActor/BI_FadeInterface.Fade Out`
  (`self.Set Material To Dynamic`)
  (bind (_direction _fade) (`Timeline|Fade` :!via `PlayFromStart` :!label _label)
    (:`Update`
      (for _array_element (`self.DynamicMeterialInstance`)
        (`MaterialInstanceDynamic.SetScalarParameterValue` _array_element "Fade" _fade)))
    (:`Finished`
      (`self.Fade Finish` _fade _fade))))

(event `/Game/Blueprints/Actors/FadeActor/BI_FadeInterface.Fade In`
  (goto _label :!via `Reverse`))

(event `self.ReceiveBeginPlay`)

(fn `Fade Finish`
  (params (A :type "Float (double-precision)") (A2 :type "Float (double-precision)"))
  (if (>= A2 1.0)
    (`self.Reset Materials`)
    (elif (<= A 0.0)
      _)))

(fn `Reset Materials`
  (for (_array_element _array_index) (`self.OriginalMaterials`)
    (`PrimitiveComponent.SetMaterial` (`self.StaticMesh`) _array_index _array_element)))

(fn `Set Material To Dynamic`
  (for (_array_element _array_index) (`self.DynamicMeterialInstance`)
    (`PrimitiveComponent.SetMaterial` (`self.StaticMesh`) _array_index _array_element)))

(fn `UserConstructionScript`
  (`KismetArrayLibrary.Array_Clear` (`self.DynamicMeterialInstance`))
  (set `self.OriginalMaterials` (`MeshComponent.GetMaterials` (`self.StaticMesh`)))
  (for _array_element (`self.FadeMaterialInstance`)
    (bind _returnvalue (`KismetMaterialLibrary.CreateDynamicMaterialInstance` _array_element))
    (`KismetArrayLibrary.Array_AddUnique` (`self.DynamicMeterialInstance`) _returnvalue)))