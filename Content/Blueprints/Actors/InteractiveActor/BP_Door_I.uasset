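; BP_Door_I is an interactable door that swings open once and has no close logic.
; QueryInteraction always allows interaction and supplies ApproachPoint's location as the approach location.
; TryInteract sets IsOpen and plays a timeline that lerps DoorLine's rotation from closed to a yawed open rotation, both cached at BeginPlay.
; Highlighting toggles custom depth on primitives tagged "Highlight", given a stencil value at BeginPlay.
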(event `self.ReceiveBeginPlay`
  (`|ExecutionSequence`
    (:`then_0`
      (`KismetArrayLibrary.Array_Clear` (`self.HighLightMeshArray`))
      (for _array_element (`self.GetComponentsByTag` "/Script/Engine.PrimitiveComponent" "Highlight")
        (`/Engine/EditorBlueprintResources/StandardMacros.IsValid` _array_element
          (:`Is Valid`
            (`KismetArrayLibrary.Array_AddUnique` (`self.HighLightMeshArray`) _array_element)
            (`PrimitiveComponent.SetCustomDepthStencilValue` _array_element 251)))))
    (:`then_1`
      (bind _output_get (set `self.ClosedRotation` (`SceneComponent.RelativeRotation` (`self.DoorLine`))))
      (set `self.OpenRotation` (`KismetMathLibrary.ComposeRotators` _output_get (`KismetMathLibrary.MakeRotator` 0.0 0.0 -100.0))))))

(event `OpenDoor`
  (bind (_direction _opendoor) (`Timeline|时间轴` :!via `PlayFromStart`)
    (:`Update`
      (`SceneComponent.K2_SetRelativeRotation` (`self.DoorLine`) (`KismetMathLibrary.RLerp` (`self.ClosedRotation`) (`self.OpenRotation`) _opendoor) false false))))

(event `HighlightInterface.HighlightActor`
  (for _array_element (`self.HighLightMeshArray`)
    (`/Engine/EditorBlueprintResources/StandardMacros.IsValid` _array_element
      (:`Is Valid`
        (`PrimitiveComponent.SetRenderCustomDepth` _array_element true)))))

(event `HighlightInterface.UnHighlightActor`
  (for _array_element (`self.HighLightMeshArray`)
    (`/Engine/EditorBlueprintResources/StandardMacros.IsValid` _array_element
      (:`Is Valid`
        (`PrimitiveComponent.SetRenderCustomDepth` _array_element false)))))

(fn `QueryInteraction`
  (params (Interactor :type "Pawn Object Reference") (OutInfo :type "AuraInteractionInfo Structure (by ref)"))
  (returns (ReturnValue :type Boolean))
  (setmembers `AuraInteractionInfo` :`StructRef` OutInfo :`bCanInteract` true :`ApproachLocation` (`SceneComponent.K2_GetComponentLocation` (`self.ApproachPoint`)) :`InteractionRange` 150.0 :`bAllowApproach` true)
  (return true))

(fn `SetMoveToLocation`
  (returns (OutDestination :type "Vector Structure"))
  (return (0.0 0.0 0.0)))

(fn `TryInteract`
  (params (Interactor :type "Pawn Object Reference"))
  (returns (ReturnValue :type Boolean))
  (if (not (`self.bIsOpen`))
    (set `self.bIsOpen` true)
    (`self.OpenDoor`)
    (return true)))

(fn `UserConstructionScript`)